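; Toy ball prop that a grabbing machine child actor picks up when the third-person character enters its trigger box, if TriggeredByPlayer is set.
; The machine starts hidden without box collision, then appears and eases each Tick toward a point below the ball's origin.
; After a short delay it closes with player grabbing disabled, Wwise sounds play, and MoveComponentTo raises the ball while the machine follows.
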(event `self.ReceiveBeginPlay`
  (bind _asgrabbing_machine (cast `GrabbingMachine` (`ChildActorComponent.ChildActor` (`self.BP_GrabbingMachine`))))
  (`PrimitiveComponent.SetCollisionEnabled` (`GrabbingMachine.BoxCollisionComponent` _asgrabbing_machine) "NoCollision")
  (`SceneComponent.SetHiddenInGame` (`GrabbingMachine.SkeletalMeshComponent` _asgrabbing_machine) true false)
  (`SceneComponent.SetHiddenInGame` (`GrabbingMachine.Decal` _asgrabbing_machine) true false))

(event `self.ReceiveTick`
  (params (DeltaSeconds :type "Float (single-precision)"))
  ;[1 1 1] Move downwards
  (if (and (`self.PickupBall`) (`self.TriggeredByPlayer`))
    (`SceneComponent.K2_SetWorldLocation` (`self.BP_GrabbingMachine`) (`KismetMathLibrary.VLerp` (`SceneComponent.K2_GetComponentLocation` (`self.BP_GrabbingMachine`)) (- (`SceneComponent.K2_GetComponentLocation` (`self.ToyballMesh`)) (0.0 0.0 400.0)) (* DeltaSeconds 5.0)) false false)))

(event `self.Box.OnComponentBeginOverlap`
  (params (OverlappedComponent :type "PrimitiveComponent Object Reference") (OtherActor :type "Actor Object Reference") (OtherComp :type "PrimitiveComponent Object Reference") (OtherBodyIndex :type Integer) (bFromSweep :type Boolean) (SweepResult :type "HitResult Structure (by ref)"))
  ;[1 1 1] Trigger overlap
  (cast `/Game/Blueprints/BP_ThirdPersonCharacter` OtherActor)
  (set `self.PickupBall` true)
  (if (`self.TriggeredByPlayer`)
    (`self.MoveUp`)
    (bind _asgrabbing_machine (cast `GrabbingMachine` (`ChildActorComponent.ChildActor` (`self.BP_GrabbingMachine`))))
    (`SceneComponent.SetHiddenInGame` (`GrabbingMachine.SkeletalMeshComponent` _asgrabbing_machine) false false)))

(event `MoveUp`
  (bind _toyballmesh (`self.ToyballMesh`))
  (`KismetSystemLibrary.Delay` 0.5)
  (bind _asgrabbing_machine (cast `GrabbingMachine` (`ChildActorComponent.ChildActor` (`self.BP_GrabbingMachine`))))
  (`GrabbingMachine.SetCanGrabPlayer` _asgrabbing_machine false)
  (`GrabbingMachine.SetClosed` _asgrabbing_machine true)
  (`AkGameObject.PostAkEvent` :`self` (`self.Audio`) :`AkEvent` "/Game/WwiseAudio/Events/Toyball/WE_Toyball_grab.WE_Toyball_grab")
  (`AkGameObject.PostAkEvent` :`self` (`self.Audio`) :`AkEvent` "/Game/WwiseAudio/Events/Toyball/WE_Toyball_rise.WE_Toyball_rise")
  (`KismetSystemLibrary.MoveComponentTo` _toyballmesh (+ (`SceneComponent.K2_GetComponentLocation` _toyballmesh) (`KismetMathLibrary.MakeVector` 0.0 0.0 (`self.DistanceToMoveUp`))) (`SceneComponent.K2_GetComponentRotation` _toyballmesh) false false 2.0))

(fn `UserConstructionScript`)