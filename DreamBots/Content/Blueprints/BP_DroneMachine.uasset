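; Drone machine actor with an animated button prompt and a screen tied to the drone it is set to possess.
; While the player overlaps its collision mesh, Tick alternates the billboard between pressed and unpressed icons, gamepad or spacebar, using a delayed DoOnce and FlipFlops.
; Once the machine reports inactive, it hides the billboard and applies a red screen material chosen by the drone's class, one time only.
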(event `self.ReceiveBeginPlay`
  (bind _asbp_third_person_character (cast `/Game/Blueprints/BP_ThirdPersonCharacter` (`GameplayStatics.GetPlayerPawn` 0)))
  (set `self.As BP Third Person Character` _asbp_third_person_character))

(event `self.ReceiveTick`
  (params (DeltaSeconds :type "Float (single-precision)"))
  (bind _billboard (`self.Billboard`))
  (`|ExecutionSequence`
    (:`then_0`
      (if (`self.PlayAnimation`)
        (`/Engine/EditorBlueprintResources/StandardMacros.DoOnce` false :!label _label
          (:`Completed`
            (if (`/Game/Blueprints/BP_ThirdPersonCharacter.IsUsingGamePad` (`self.As BP Third Person Character`))
              (`/Engine/EditorBlueprintResources/StandardMacros.FlipFlop`
                (:`A`
                  (`BillboardComponent.SetSprite` _billboard "/Game/ArtAssets/UI_Icons/T_Icon_Controller_Button.T_Icon_Controller_Button"))
                (:`B`
                  (`BillboardComponent.SetSprite` _billboard "/Game/ArtAssets/UI_Icons/T_Icon_Controller_Button_Pressed.T_Icon_Controller_Button_Pressed")))
              (else
                (`/Engine/EditorBlueprintResources/StandardMacros.FlipFlop`
                  (:`A`
                    (`BillboardComponent.SetSprite` _billboard "/Game/ArtAssets/UI_Icons/T_Icon_Spacebar_Pressed.T_Icon_Spacebar_Pressed"))
                  (:`B`
                    (`BillboardComponent.SetSprite` _billboard "/Game/ArtAssets/UI_Icons/T_Icon_Spacebar_New.T_Icon_Spacebar_New")))))
            (`KismetSystemLibrary.Delay` 0.5)
            (goto _label :!via `Reset`)))))
    (:`then_1`
      ;[1 1 1] Disable Screen
      (if (not (`self.GetDroneMachineActivity`))
        (`/Engine/EditorBlueprintResources/StandardMacros.DoOnce` false
          (:`Completed`
            (`self.DisableSpacebar`)
            (`self.DisableScreen`)))))))

(event `self.CollisionMesh.OnComponentBeginOverlap`
  (params (OverlappedComponent :type "PrimitiveComponent Object Reference") (OtherActor :type "Actor Object Reference") (OtherComp :type "PrimitiveComponent Object Reference") (OtherBodyIndex :type Integer) (bFromSweep :type Boolean) (SweepResult :type "HitResult Structure (by ref)"))
  ;[1 1 1] Overlap
  (if (== OtherActor (`self.As BP Third Person Character`))
    (set `self.PlayAnimation` true)))

(event `self.CollisionMesh.OnComponentEndOverlap`
  (params (OverlappedComponent :type "PrimitiveComponent Object Reference") (OtherActor :type "Actor Object Reference") (OtherComp :type "PrimitiveComponent Object Reference") (OtherBodyIndex :type Integer))
  ;[1 1 1] Overlap
  (cast `/Game/Blueprints/BP_ThirdPersonCharacter` OtherActor)
  (set `self.PlayAnimation` false))

(fn `DisableScreen`
  (if (== (`GameplayStatics.GetObjectClass` (`self.DroneToPossess`)) "/Game/Blueprints/BP_ShootingDrone.BP_ShootingDrone_C")
    (`PrimitiveComponent.SetMaterial` (`self.DroneMachineMesh`) 3 "/Game/ArtAssets/Shader/MXI_DroneScreen_Red.MXI_DroneScreen_Red")
    (else
      (`PrimitiveComponent.SetMaterial` (`self.DroneMachineMesh`) 3 "/Game/ArtAssets/Shader/MXI_DroneScreen_2_Red.MXI_DroneScreen_2_Red"))))

(fn `DisableSpacebar`
  (`SceneComponent.SetHiddenInGame` (`self.Billboard`) true false))

(fn `UserConstructionScript`)