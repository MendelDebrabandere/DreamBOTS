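; BP_MazeConsole is a maze console that shows an animated button prompt while the player character overlaps its collision mesh.
; Overlap events toggle a flag that Tick reads, flip-flopping billboard sprites between normal and pressed every half second, using gamepad or spacebar icons to match the character's input.
; Tick also polls console activity and, once inactive, hides the prompt billboard and static mesh and swaps the screen material, one time only.
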(event `self.ReceiveBeginPlay`
  (bind _asbp_third_person_character (cast `/Game/Blueprints/BP_ThirdPersonCharacter` (`GameplayStatics.GetPlayerPawn` 0)))
  (set `self.As BP Third Person Character` _asbp_third_person_character))

(event `self.ReceiveTick`
  (params (DeltaSeconds :type "Float (single-precision)"))
  (bind _billboard (`self.Billboard`))
  (bind _billboard_2 (`self.Billboard`))
  (`|ExecutionSequence`
    (:`then_1`
      (if (`self.PlayAnimation`)
        (`/Engine/EditorBlueprintResources/StandardMacros.DoOnce` false :!label _label
          (:`Completed`
            (if (`/Game/Blueprints/BP_ThirdPersonCharacter.IsUsingGamePad` (`self.As BP Third Person Character`))
              (`/Engine/EditorBlueprintResources/StandardMacros.FlipFlop`
                (:`A`
                  (`BillboardComponent.SetSprite` _billboard "/Game/ArtAssets/UI_Icons/T_Icon_Controller_Button.T_Icon_Controller_Button"))
                (:`B`
                  (`BillboardComponent.SetSprite` _billboard "/Game/ArtAssets/UI_Icons/T_Icon_Controller_Button_Pressed.T_Icon_Controller_Button_Pressed")))
              (else
                (`/Engine/EditorBlueprintResources/StandardMacros.FlipFlop`
                  (:`A`
                    (`BillboardComponent.SetSprite` _billboard_2 "/Game/ArtAssets/UI_Icons/T_Icon_Spacebar_New.T_Icon_Spacebar_New"))
                  (:`B`
                    (`BillboardComponent.SetSprite` _billboard_2 "/Game/ArtAssets/UI_Icons/T_Icon_Spacebar_Pressed.T_Icon_Spacebar_Pressed")))))
            (`KismetSystemLibrary.Delay` 0.5)
            (goto _label :!via `Reset`)))))
    (:`then_2`
      ;[1 1 1] Deactivate console
      (if (not (`self.GetMazeConsoleActivity`))
        (`/Engine/EditorBlueprintResources/StandardMacros.DoOnce` false
          (:`Completed`
            (`self.DeactivateSpacebar`)
            (`self.DisableScreen`)))))))

(event `self.CollisionMesh.OnComponentBeginOverlap`
  (params (OverlappedComponent :type "PrimitiveComponent Object Reference") (OtherActor :type "Actor Object Reference") (OtherComp :type "PrimitiveComponent Object Reference") (OtherBodyIndex :type Integer) (bFromSweep :type Boolean) (SweepResult :type "HitResult Structure (by ref)"))
  (cast `/Game/Blueprints/BP_ThirdPersonCharacter` OtherActor)
  (set `self.PlayAnimation` true))

(event `self.CollisionMesh.OnComponentEndOverlap`
  (params (OverlappedComponent :type "PrimitiveComponent Object Reference") (OtherActor :type "Actor Object Reference") (OtherComp :type "PrimitiveComponent Object Reference") (OtherBodyIndex :type Integer))
  (cast `/Game/Blueprints/BP_ThirdPersonCharacter` OtherActor)
  (set `self.PlayAnimation` false))

(fn `DeactivateSpacebar`
  (`SceneComponent.SetHiddenInGame` (`self.Billboard`) true false)
  (`SceneComponent.SetHiddenInGame` (`self.StaticMesh`) true false))

(fn `DisableScreen`
  (`PrimitiveComponent.SetMaterial` (`self.ToyballConsoleMesh`) 1 "/Game/ArtAssets/Shader/MXI_Claw_Screen_2.MXI_Claw_Screen_2"))

(fn `UserConstructionScript`)