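; BP_ShootingDrone is a player-controllable drone that shows an animated button prompt billboard while the player pawn is of its class.
; When player-controlled, Tick overrides the audio listener onto DroneRoot, offsetting rotation to follow FollowCamera.
; A self-resetting DoOnce with Delay and FlipFlop alternates pressed and released sprites.
; Any key press switches the prompt between spacebar and gamepad icons based on the input device.
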(event `self.ReceiveBeginPlay`)

(event `self.ReceiveTick`
  (params (DeltaSeconds :type "Float (single-precision)"))
  (bind _billboard (`self.Billboard`))
  (bind (_returnvalue_roll _returnvalue_pitch _returnvalue_yaw) (`KismetMathLibrary.BreakRotator` (`KismetMathLibrary.ComposeRotators` (* (`self.K2_GetActorRotation`) -1.0) (`SceneComponent.K2_GetComponentRotation` (`self.FollowCamera`)))))
  (`|ExecutionSequence`
    (:`then_0`
      ;[1 1 1] Overriding audio listener
      (if (`self.IsPlayerControlled`)
        (`PlayerController.SetAudioListenerOverride` (`GameplayStatics.GetPlayerController` 0) (`self.DroneRoot`) (0.0 0.0 0.0) (`KismetMathLibrary.MakeRotator` _returnvalue_roll _returnvalue_pitch (+ _returnvalue_yaw 0.0)))))
    (:`then_1`
      ;[1 1 1] Spacebar Animation
      (`/Engine/EditorBlueprintResources/StandardMacros.DoOnce` false :!label _label
        (:`Completed`
          (if (`self.UsingGamePad`)
            (`/Engine/EditorBlueprintResources/StandardMacros.FlipFlop`
              (:`A`
                ;[1 1 1] Swap Out sprites
                (`BillboardComponent.SetSprite` _billboard "/Game/ArtAssets/UI_Icons/T_Icon_Controller_Button.T_Icon_Controller_Button"))
              (:`B`
                (`BillboardComponent.SetSprite` _billboard "/Game/ArtAssets/UI_Icons/T_Icon_Controller_Button_Pressed.T_Icon_Controller_Button_Pressed")))
            (else
              (`/Engine/EditorBlueprintResources/StandardMacros.FlipFlop`
                (:`A`
                  (`BillboardComponent.SetSprite` _billboard "/Game/ArtAssets/UI_Icons/T_Icon_Spacebar_Pressed.T_Icon_Spacebar_Pressed"))
                (:`B`
                  (`BillboardComponent.SetSprite` _billboard "/Game/ArtAssets/UI_Icons/T_Icon_Spacebar_New.T_Icon_Spacebar_New")))))
          (`KismetSystemLibrary.Delay` 0.7)
          (goto _label :!via `Reset`))))
    (:`then_2`
      ;[1 1 1] Show/Hide
      (if (== (`GameplayStatics.GetObjectClass` (`GameplayStatics.GetPlayerPawn` 0)) (`GameplayStatics.GetObjectClass` self))
        (`self.ActivateSpacebar`)
        (else
          (`self.DisableSpacebar`))))))

(event `Key|AnyKey` :consume false
  (params (Key :type "Key Structure"))
  (:`Pressed`
    (if (`KismetInputLibrary.Key_IsGamepadKey` Key)
      (set `self.UsingGamePad` true)
      (else
        (set `self.UsingGamePad` false)))))

(fn `ActivateSpacebar`
  (`SceneComponent.SetHiddenInGame` (`self.Billboard`) false false))

(fn `DisableSpacebar`
  (`SceneComponent.SetHiddenInGame` (`self.Billboard`) true false))

(fn `UserConstructionScript`)