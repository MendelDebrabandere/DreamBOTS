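; BP_PoisonFloor is a poison floor that records where the character has been by painting into a render target.
; DoCharacterLineTrace traces down from the character against CleaningPlatform objects and, on hitting a poison floor, passes the collision UV to DrawToRT.
; The render target resets to black on BeginPlay and EndPlay, while ClearFloor fills it white in one step.
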(event `self.ClearFloor`
  (`KismetRenderingLibrary.ClearRenderTarget2D` (`self.PoisonRenderTarget`) (struct :`R` 1.0 :`G` 1.0 :`B` 1.0 :`A` 1.0)))

(event `self.ReceiveBeginPlay`
  ;[1 1 1] Clearing the color of the rendertarget
  (`KismetRenderingLibrary.ClearRenderTarget2D` (`self.PoisonRenderTarget`)))

(event `self.ReceiveEndPlay`
  (params (EndPlayReason :type "EEndPlayReason Enum" :default "Destroyed"))
  (`KismetRenderingLibrary.ClearRenderTarget2D` (`self.PoisonRenderTarget`)))

(event `self.DoCharacterLineTrace`
  (bind _returnvalue (`self.K2_GetActorLocation` (`self.Character`)))
  ;[1 1 1] Do line trace
  (bind (_outhit _returnvalue_2) (`KismetSystemLibrary.LineTraceSingleForObjects` :`Start` (+ _returnvalue (0.0 0.0 100.0)) :`End` (+ _returnvalue (`KismetMathLibrary.MakeVector` 0.0 0.0 -1000.0)) :`ObjectTypes` (`self.CleaningPlatform`) :`bIgnoreSelf` false))
  (if _returnvalue_2
    ;[1 1 1] If the hit actor is the poison floor, paint on it
    (cast `/Game/Blueprints/BP_PoisonFloor` (`.HitActor` (`GameplayStatics.BreakHitResult` _outhit)))
    (`self.DrawToRT` (`GameplayStatics.FindCollisionUV` _outhit))))

(fn `UserConstructionScript`)