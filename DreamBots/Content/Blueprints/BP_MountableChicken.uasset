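; Rideable chicken that shows a spacebar prompt when the third-person character is near and speeds up while mounted.
; Mount and dismount events set the speed of its moving actor, animation rate, prompt and Wwise audio.
; Tick lerps mounted speed toward a cap, passing it to the moving actor.
; Rising speed steps through three one-way stages that intensify fire, smoke, animation and engine-load audio, ending in an ignite sound and top speed.
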(event `self.ReceiveBeginPlay`
  (`|ExecutionSequence`
    (:`then_0`
      (bind _asbp_third_person_character (cast `/Game/Blueprints/BP_ThirdPersonCharacter` (`GameplayStatics.GetPlayerPawn` 0)))
      (set `self.As BP Third Person Character` _asbp_third_person_character)
      (`SceneComponent.SetHiddenInGame` (`self.Billboard`) true false))
    (:`then_1`
      (`AkGameObject.SetRTPCValue` (`self.Audio`) "/Game/WwiseAudio/RTPC/RTPC_Load.RTPC_Load" 0.0 0 "")
      (`AkGameObject.PostAkEvent` :`self` (`self.Audio`) :`AkEvent` "/Game/WwiseAudio/Events/Kippie/WE_Start_clucking.WE_Start_clucking")
      (`NiagaraComponent.SetVariableFloat` (`self.NS_SmokeTrail`) "SpawnRate" 8.5)
      (`NiagaraComponent.SetVariableFloat` (`self.NS_SmokeTrail`) "Size" 1.0))))

(event `self.CollisionBox.OnComponentBeginOverlap`
  (params (OverlappedComponent :type "PrimitiveComponent Object Reference") (OtherActor :type "Actor Object Reference") (OtherComp :type "PrimitiveComponent Object Reference") (OtherBodyIndex :type Integer) (bFromSweep :type Boolean) (SweepResult :type "HitResult Structure (by ref)"))
  (cast `/Game/Blueprints/BP_ThirdPersonCharacter` OtherActor)
  ;[1 1 1] Show when close to kippie
  (`SceneComponent.SetHiddenInGame` (`self.Billboard`) false false))

(event `self.CollisionBox.OnComponentEndOverlap`
  (params (OverlappedComponent :type "PrimitiveComponent Object Reference") (OtherActor :type "Actor Object Reference") (OtherComp :type "PrimitiveComponent Object Reference") (OtherBodyIndex :type Integer))
  (cast `/Game/Blueprints/BP_ThirdPersonCharacter` OtherActor)
  ;[1 1 1] Hide when not close
  (`SceneComponent.SetHiddenInGame` (`self.Billboard`) true false))

(event `self.Mounted`
  (bind _returnvalue (`self.GetMovingActor`))
  (set `self.IsMounted` true)
  (`AkGameObject.SetRTPCValue` (`self.Audio`) "/Game/WwiseAudio/RTPC/RTPC_Load.RTPC_Load" 100.0 200 "")
  (set `self.CurrentSpeed` (`self.SpeedWhenMounted`))
  (`/Engine/EditorBlueprintResources/StandardMacros.IsValid` _returnvalue
    (:`Is Valid`
      (`MovingActor.SetSpeed` _returnvalue (`self.SpeedWhenMounted`))
      (set `SkeletalMeshComponent.GlobalAnimRateScale` (`self.SpeedWhenMounted`) (`self.SkeletalMesh`))
      (`AkGameObject.PostAkEvent` :`self` (`self.Audio`) :`AkEvent` "/Game/WwiseAudio/Events/Kippie/WE_Start_fast_kippie.WE_Start_fast_kippie")
      ;[1 1 1] Set spacebar hidden when riding
      (if (`DreamBotsCharacter.GetIsRiding` (`self.As BP Third Person Character`))
        (`SceneComponent.SetHiddenInGame` (`self.Billboard`) true false)
        (set `self.Stage` 0)
        (`NiagaraComponent.SetVariableFloat` (`self.NS_SmokeTrail`) "SpawnRate" 8.5)
        (`NiagaraComponent.SetVariableFloat` (`self.NS_SmokeTrail`) "Size" 1.0)))))

(event `self.Dismount`
  (bind _returnvalue (`self.GetMovingActor`))
  (set `self.IsMounted` false)
  (`AkGameObject.SetRTPCValue` (`self.Audio`) "/Game/WwiseAudio/RTPC/RTPC_Load.RTPC_Load" 0.0 200 "")
  (`/Engine/EditorBlueprintResources/StandardMacros.IsValid` _returnvalue
    (:`Is Valid`
      (`MovingActor.SetSpeed` _returnvalue 1.0)
      (set `self.CurrentSpeed` 3.0)
      (set `SkeletalMeshComponent.GlobalAnimRateScale` 1.0 (`self.SkeletalMesh`))
      (`AkGameObject.PostAkEvent` :`self` (`self.Audio`) :`AkEvent` "/Game/WwiseAudio/Events/Kippie/WE_Stop_fast_kippie.WE_Stop_fast_kippie")
      ;[1 1 1] Set spacebar visable when riding
      (if (`DreamBotsCharacter.GetIsRiding` (`self.As BP Third Person Character`))
        (`SceneComponent.SetHiddenInGame` (`self.Billboard`) false false)
        (set `self.Stage` 0)
        (`ActorComponent.Deactivate` (`self.FireParticles`))
        (`NiagaraComponent.SetVariableFloat` (`self.NS_SmokeTrail`) "SpawnRate" 8.5)
        (`NiagaraComponent.SetVariableFloat` (`self.NS_SmokeTrail`) "Size" 1.0)))))

(event `self.ReceiveTick`
  (params (DeltaSeconds :type "Float (single-precision)"))
  (bind _returnvalue (`self.GetMovingActor`))
  (set `self.Delta Seconds` DeltaSeconds)
  (`|ExecutionSequence`
    (:`then_0`
      ;[1 1 1] Update speed
      (if (`self.IsMounted`)
        (set `self.CurrentSpeed` (`KismetMathLibrary.Lerp` (`self.CurrentSpeed`) 5.5 (* (`self.Delta Seconds`) (`self.Acceleration`))))
        (`/Engine/EditorBlueprintResources/StandardMacros.IsValid` _returnvalue
          (:`Is Valid`
            (`MovingActor.SetSpeed` _returnvalue (`self.CurrentSpeed`))))))
    (:`then_1`
      ;[1 1 1] Stage 1
      (if (== (`self.Stage`) 0)
        (if (> (`self.CurrentSpeed`) 3.5)
          (`ActorComponent.Activate` (`self.FireParticles`) false)
          (`NiagaraComponent.SetVariableFloat` (`self.FireParticles`) "SpawnRate" 150.0)
          (set `self.Stage` 1)
          (set `SkeletalMeshComponent.GlobalAnimRateScale` (`self.CurrentSpeed`) (`self.SkeletalMesh`)))))
    (:`then_2`
      ;[1 1 1] Stage 2
      (if (== (`self.Stage`) 1)
        (if (> (`self.CurrentSpeed`) 4.0)
          (`NiagaraComponent.SetVariableFloat` (`self.FireParticles`) "SpawnRate" 250.0)
          (set `self.Stage` 2)
          (set `SkeletalMeshComponent.GlobalAnimRateScale` (`self.CurrentSpeed`) (`self.SkeletalMesh`))
          (`NiagaraComponent.SetVariableFloat` (`self.NS_SmokeTrail`) "SpawnRate" 12.0)
          (`AkGameObject.SetRTPCValue` (`self.Audio`) "/Game/WwiseAudio/RTPC/RTPC_Load.RTPC_Load" 75.0 200 ""))))
    (:`then_3`
      ;[1 1 1] Stage 3
      (if (== (`self.Stage`) 2)
        (if (> (`self.CurrentSpeed`) 4.5)
          (`NiagaraComponent.SetVariableFloat` (`self.FireParticles`) "SpawnRate" 400.0)
          (set `self.Stage` 3)
          (`AkGameObject.PostAkEvent` :`self` (`self.Audio`) :`AkEvent` "/Game/WwiseAudio/Events/Kippie/WE_Kippie_ignite.WE_Kippie_ignite")
          (set `self.CurrentSpeed` 5.5)
          (set `SkeletalMeshComponent.GlobalAnimRateScale` (`self.CurrentSpeed`) (`self.SkeletalMesh`))
          (`NiagaraComponent.SetVariableFloat` (`self.NS_SmokeTrail`) "SpawnRate" 30.0)
          (`NiagaraComponent.SetVariableFloat` (`self.NS_SmokeTrail`) "Size" 2.0)
          (`AkGameObject.SetRTPCValue` (`self.Audio`) "/Game/WwiseAudio/RTPC/RTPC_Load.RTPC_Load" 100.0 200 ""))))))

(fn `UserConstructionScript`)