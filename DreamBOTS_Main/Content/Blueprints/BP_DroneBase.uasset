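; Base Blueprint for a drone that adds a pause-screen HUD and controls audio listening while player-controlled.
; On BeginPlay it creates the HUD_PauseScreen widget, stores a reference and adds it to the viewport.
; Each tick under player control, it overrides player 0's audio listener, attaching it to DroneRoot.
; The listener's rotation combines the negated actor rotation with the FollowCamera's world rotation, with roll flipped, to offset it toward the camera's view.
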(event `self.ReceiveBeginPlay`
  (bind _returnvalue (`|CreateWidget` "/Game/Blueprints/UI/HUD_PauseScreen.HUD_PauseScreen_C"))
  (bind _output_get (set `self.HUD_PauseScreen_Ref` _returnvalue))
  (`UserWidget.AddToViewport` _output_get 0))

(event `self.ReceiveTick`
  (params (DeltaSeconds :type "Float (single-precision)"))
  (bind (_returnvalue_roll _returnvalue_pitch _returnvalue_yaw) (`KismetMathLibrary.BreakRotator` (`KismetMathLibrary.ComposeRotators` (* (`self.K2_GetActorRotation`) -1.0) (`SceneComponent.K2_GetComponentRotation` (`self.FollowCamera`)))))
  ;[1 1 1] Overriding audio listener
  (if (`self.IsPlayerControlled`)
    (`PlayerController.SetAudioListenerOverride` (`GameplayStatics.GetPlayerController` 0) (`self.DroneRoot`) (0.0 0.0 0.0) (`KismetMathLibrary.MakeRotator` (* _returnvalue_roll -1.0) _returnvalue_pitch _returnvalue_yaw))))

(fn `UserConstructionScript`)