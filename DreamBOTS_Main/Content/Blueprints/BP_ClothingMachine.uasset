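; BP_ClothingMachine is a clothing machine actor that starts its Wwise audio when play begins.
; BeginPlay posts the associated AkEvent on nine components, one named Main and eight numbered ones, with no callbacks requested.
; Overlap, Tick and the construction script hold no logic.
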(event `self.ReceiveBeginPlay`
  (`AkGameObject.PostAssociatedAkEvent` :`self` (`self.Main`))
  (`AkGameObject.PostAssociatedAkEvent` :`self` (`self.1`))
  (`AkGameObject.PostAssociatedAkEvent` :`self` (`self.2`))
  (`AkGameObject.PostAssociatedAkEvent` :`self` (`self.3`))
  (`AkGameObject.PostAssociatedAkEvent` :`self` (`self.4`))
  (`AkGameObject.PostAssociatedAkEvent` :`self` (`self.5`))
  (`AkGameObject.PostAssociatedAkEvent` :`self` (`self.6`))
  (`AkGameObject.PostAssociatedAkEvent` :`self` (`self.7`))
  (`AkGameObject.PostAssociatedAkEvent` :`self` (`self.8`)))

(fn `UserConstructionScript`)