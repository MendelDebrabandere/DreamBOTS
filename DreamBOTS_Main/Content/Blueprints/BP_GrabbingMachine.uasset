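; BP_GrabbingMachine is a grabbing machine Blueprint whose vertical arm stretches to reach a fixed height reference.
; On BeginPlay it stores the world location of MaxVertSize, or disables arm resizing if its owner is a BP_ToyBall.
; While resizing is enabled, Tick sets the ArmExtender's Z scale from its vertical distance to that stored point, leaving X and Y scale unchanged.
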(event `self.ReceiveBeginPlay`
  (cast `/Game/Blueprints/BP_ToyBall` (`self.GetOwner`)
    (:`then`
      (set `self.bShouldSetVertSize` false))
    (:`CastFailed`
      (set `self.MaxVertLocationVariab` (`SceneComponent.K2_GetComponentLocation` (`self.MaxVertSize`))))))

(event `self.ReceiveTick`
  (params (DeltaSeconds :type "Float (single-precision)"))
  (bind _armextender (`self.ArmExtender`))
  (bind (_maxvertlocationvariab_x _maxvertlocationvariab_y _maxvertlocationvariab_z) (`KismetMathLibrary.BreakVector` (`self.MaxVertLocationVariab`)))
  (bind (_returnvalue_x _returnvalue_y _returnvalue_z) (`KismetMathLibrary.BreakVector` (`SceneComponent.K2_GetComponentLocation` (`self.ArmExtender`))))
  (bind (_relativescale3d_x _relativescale3d_y) (`KismetMathLibrary.BreakVector` (`SceneComponent.RelativeScale3D` _armextender)))
  (if (`self.bShouldSetVertSize`)
    (`SceneComponent.SetRelativeScale3D` _armextender (`KismetMathLibrary.MakeVector` _relativescale3d_x _relativescale3d_y (/ (`KismetMathLibrary.Abs` (- _returnvalue_z _maxvertlocationvariab_z)) 100.0)))))

(fn `UserConstructionScript`)